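; BP_PlayerPawn is a player pawn that rolls a sphere using physics torque.
; The forward/backward and right/left axis inputs apply torque around the world Y and X axes, scaled by TorqueForce.
; Torque is applied as an acceleration change, so the roll response is independent of the sphere's mass.
; BeginPlay starts a two-second camera fade in from black.
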(event EventBeginPlay
  (CameraFades|StartCameraFade (Game|GetPlayerCameraManager 0) 1.0 0.0 2.0 "(R=0.000000,G=0.000000,B=0.000000,A=1.000000)" false false))

(event Collision|EventActorBeginOverlap
  (params (OtherActor :type Actor%20Object%20Reference)))

(event EventTick
  (params (DeltaSeconds :type Float%20%28single-precision%29)))

(event Input|AxisEvents|InputAxisMoveForwards/Backwards
  (params (AxisValue :type Float%20%28single-precision%29))
  (Class|PrimitiveComponent|AddTorqueinRadians (Variables|Default|GetShape_Sphere) (Math|Vector|MakeVector 0.0 (* AxisValue (Variables|Default|GetTorque_Force)) 0.0) "None" true))

(event Input|AxisEvents|InputAxisMoveRight/Left
  (params (AxisValue :type Float%20%28single-precision%29))
  (Class|PrimitiveComponent|AddTorqueinRadians (Variables|Default|GetShape_Sphere) (Math|Vector|MakeVector (* AxisValue (Variables|Default|GetTorque_Force)) 0.0 0.0) "None" true))

(fn ConstructionScript)