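; BP_Cannon is an automatic cannon actor that repeatedly fires BP_Projectile from BeginPlay onward.
; After a FireRate delay, it spawns the projectile at the ProjectileSpawnPoint's world location and rotation, scaled by ProjectileScale.
; CannonTimeline then moves the barrel along its relative Y axis.
; The timeline's Cannon Fired event track loops back to the delay, sustaining the firing cycle without Tick or a timer.
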(event EventBeginPlay
  (bind _projectile_spawn_point (Variables|Default|GetProjectile%20Spawn%20Point))
  (Utilities|FlowControl|Delay (Variables|CannonProperties|GetFire%20Rate) :!label _label)
  (Game|SpawnActorfromClass "/Game/Blueprints/Actors/BP_Projectile.BP_Projectile_C" (Math|Transform|MakeTransform (Transformation|GetWorldLocation _projectile_spawn_point) (Transformation|GetWorldRotation _projectile_spawn_point) (Math|Conversions|ToVector(Float) (Variables|CannonProperties|GetProjectile%20Scale))) "Undefined" 0 0)
  (bind _cannon_barrel_location (Timeline|Cannon%20Timeline PlayFromStart)
    (:Update
      (Transformation|SetRelativeLocation (Variables|Default|GetCannon%20Barrel) (Math|Vector|MakeVector 0.0 _cannon_barrel_location 0.0) false false))
    (:Cannon%20Fired
      (goto _label))))

(fn ConstructionScript)